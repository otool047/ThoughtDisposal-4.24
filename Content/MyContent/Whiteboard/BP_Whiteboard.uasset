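; Whiteboard actor that lets marker strokes be drawn onto a shared render target at runtime.
; On BeginPlay it creates a dynamic instance of the marker material and clears the render target to black, clearing it again on EndPlay.
; DrawOnWhiteboard passes a 2D location into the material's DrawLocation parameter, then draws that material into the render target to add the mark.
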(event Custom|DrawOnWhiteboard
  (params (LocationToDraw :type Vector%202D%20Structure))
  (bind _whiteboardmarker_mi (Variables|Default|GetWhiteboardMarker_MI))
  (Rendering|Material|SetVectorParameterValue _whiteboardmarker_mi "DrawLocation" (Math|Conversions|ToLinearColor(Vector) (Math|Conversions|ToVector(Vector2D) LocationToDraw)) :!class /Script/Engine.MaterialInstanceDynamic)
  (Rendering|DrawMaterialtoRenderTarget "/Game/MyContent/Whiteboard/RT_Whiteboard.RT_Whiteboard" _whiteboardmarker_mi))

(event EventBeginPlay
  (bind _returnvalue (Rendering|Material|CreateDynamicMaterialInstance "/Game/MyContent/Whiteboard/M_WhiteboardMarker.M_WhiteboardMarker" "None" :!class /Script/Engine.KismetMaterialLibrary))
  (Variables|Default|SetWhiteboardMarker_MI _returnvalue)
  (Rendering|ClearRenderTarget2D "/Game/MyContent/Whiteboard/RT_Whiteboard.RT_Whiteboard"))

(event Collision|EventActorBeginOverlap
  (params (OtherActor :type Actor%20Object%20Reference)))

(event EventTick
  (params (DeltaSeconds :type Float%20%28single-precision%29)))

(event EventEndPlay
  (params (EndPlayReason :type EEndPlayReason%20Enum :default "Destroyed"))
  (Rendering|ClearRenderTarget2D "/Game/MyContent/Whiteboard/RT_Whiteboard.RT_Whiteboard"))

(fn ConstructionScript)