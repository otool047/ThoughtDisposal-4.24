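; BP_Wolf is a wolf pawn that follows the first MotionControllerPawn, looked up every Tick.
; Beyond StopDistance it uses AI MoveToActor and takes its yaw from the look-at toward its previous-frame position.
; Within that distance, a multiplier eases FloatingPawnMovement's max speed to zero over about a second.
; Each frame a downward Visibility trace, with debug drawing, snaps the wolf onto the surface below.
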(event EventTick
  (params (DeltaSeconds :type Float%20%28single-precision%29))
  (bind _outactors (Actor|GetAllActorsOfClass "/Game/VirtualRealityBP/Blueprints/MotionControllerPawn.MotionControllerPawn_C"))
  (Variables|Default|SetPlayer (Utilities|Array|Get(acopy) _outactors))
  (CallFunction|MoveTowardsPlayer DeltaSeconds)
  (CallFunction|CorrectZ)
  (Variables|Default|SetLastPos (Transformation|GetActorLocation)))

(fn ConstructionScript)

(fn MoveTowardsPlayer
  (params (Delta%20Time :type Float%20%28single-precision%29))
  (bind _self self)
  (bind _player (Variables|Default|GetPlayer))
  (bind _stopdistance (Variables|Default|GetStopDistance))
  (bind _returnvalue (Transformation|GetDistanceTo _self _player))
  (bind _returnvalue_2 (> _returnvalue _stopdistance))
  (CallFunction|UpdateMovementSpeed _returnvalue_2)
  (if _returnvalue_2
    (AI|Navigation|MovetoActor (AI|GetAIController _self) _player -1.0 false true false 0)
    (Transformation|SetActorRotation (Math|Rotator|MakeRotator 0.0 0.0 (.Yaw (Math|Rotator|BreakRotator (Math|Rotator|FindLookatRotation (Transformation|GetActorLocation) (Variables|Default|GetLastPos))))))))

(fn CorrectZ
  (bind _returnvalue (Transformation|GetActorLocation))
  (bind (_outhit _returnvalue_2) (Collision|LineTraceByChannel _returnvalue (- _returnvalue "0, 0,1000.000000") "TraceTypeQuery1" false 0 "ForOneFrame"))
  (if _returnvalue_2
    (Transformation|SetActorLocation (.Location (Collision|BreakHitResult _outhit)) false false)))

(fn UpdateMovementSpeed
  (params (Moving :type Boolean))
  (if (not Moving)
    (Variables|Default|SetMovementMult (Math|Float|Clamp(Float) (- (Variables|Default|GetMovementMult) (Utilities|Time|GetWorldDeltaSeconds))))
    (else
      (Variables|Default|SetMovementMult 1.0)))
  (Variables|/Script/Engine.FloatingPawnMovement|SetMaxSpeed (Variables|Default|GetFloatingPawnMovement) (* (Variables|Default|GetMovementMult) (Variables|Default|GetMovementSpeed))))